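; Player controller that handles grabbing, interacting, crouching and pausing for the player character.
; Grab traces from the L1_Character camera, messages BPI_Grab objects and releases them when input completes; Move start nudges a held BP_PhysDoor.
; Interact sends a message to actors hit by a shorter camera trace.
; Escape and P duplicate the WBP_PauseMenu toggle, and the HG_InputMapping setup is never executed.
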(event `EnhancedInput|/Game/Inputs/InputActions/IA_Grab`
  (params (ActionValue :type Boolean) (ElapsedSeconds :type "Float (double-precision)") (TriggeredSeconds :type "Float (double-precision)") (InputAction :type "InputAction Object Reference" :default "/Game/Inputs/InputActions/IA_Grab.IA_Grab"))
  (bind _grabbedobject (`self.GrabbedObject`))
  (:`Started`
    (bind _hitactor (`self.LineTrace` 350.0))
    (set `self.GrabbedObject` _hitactor)
    (if (and (`KismetSystemLibrary.IsValid` _hitactor) (`KismetSystemLibrary.DoesImplementInterface` _hitactor "/Game/Blueprints/Interfaces/BPI_Grab.BPI_Grab_C"))
      (message `/Game/Blueprints/Interfaces/BPI_Grab.Grab Object` (`self.GrabbedObject`))))
  (:`Completed`
    (`/Engine/EditorBlueprintResources/StandardMacros.IsValid` _grabbedobject
      (:`Is Valid`
        (message `/Game/Blueprints/Interfaces/BPI_Grab.ReleaseObject` _grabbedobject)
        (set `self.GrabbedObject` null)))))

(event `EnhancedInput|/Game/Inputs/InputActions/IA_Move`
  (params (ActionValue :type "Vector2D Structure") (ElapsedSeconds :type "Float (double-precision)") (TriggeredSeconds :type "Float (double-precision)") (InputAction :type "InputAction Object Reference" :default "/Game/Inputs/InputActions/IA_Move.IA_Move"))
  (:`Started`
    (bind _asbp_phys_door (cast `/Game/Blueprints/Actors/Grabbable/BP_PhysDoor` (`self.GrabbedObject`)))
    (`/Game/Blueprints/Actors/Grabbable/BP_PhysDoor.MoveDoor` _asbp_phys_door 4.0)))

(event `EnhancedInput|/Game/Inputs/InputActions/IA_Crouch`
  (params (ActionValue :type Boolean) (ElapsedSeconds :type "Float (double-precision)") (TriggeredSeconds :type "Float (double-precision)") (InputAction :type "InputAction Object Reference" :default "/Game/Inputs/InputActions/IA_Crouch.IA_Crouch"))
  (:`Started`
    (`Character.Crouch` (`GameplayStatics.GetPlayerCharacter` 0)))
  (:`Completed`
    (`Character.UnCrouch` (`GameplayStatics.GetPlayerCharacter` 0))))

(event `EnhancedInput|/Game/Inputs/InputActions/IA_Interact`
  (params (ActionValue :type Boolean) (ElapsedSeconds :type "Float (double-precision)") (TriggeredSeconds :type "Float (double-precision)") (InputAction :type "InputAction Object Reference" :default "/Game/Inputs/InputActions/IA_Interact.IA_Interact"))
  (:`Started`
    (bind _asl1_character (cast `/Game/Blueprints/Level1/L1_Character` (`GameplayStatics.GetPlayerCharacter` 0)))
    (bind _camera (`/Game/Blueprints/Level1/L1_Character.Camera` _asl1_character))
    (bind _returnvalue (`SceneComponent.K2_GetComponentLocation` _camera))
    (bind (_outhit _returnvalue_2) (`KismetSystemLibrary.LineTraceSingle` _returnvalue (+ _returnvalue (* (`KismetMathLibrary.GetForwardVector` (`SceneComponent.K2_GetComponentRotation` _camera)) 200.0)) "TraceTypeQuery1"))
    (if _returnvalue_2
      (message `/Game/Blueprints/Interfaces/BPI_Interaction.Interact` (`.HitActor` (`GameplayStatics.BreakHitResult` _outhit))))))

(event `Key|Escape`
  (params (Key :type "Key Structure"))
  (:`Pressed`
    (if (`self.IsPauseMenuOpen`)
      (set `self.IsPauseMenuOpen` false)
      (`Widget.RemoveFromParent` (`self.PauseMenuREF`))
      (set `self.PauseMenuREF` null)
      (`WidgetBlueprintLibrary.SetInputMode_GameOnly` self)
      (set `self.bShowMouseCursor` false)
      (`GameplayStatics.SetGamePaused` false)
      (else
        (set `self.IsPauseMenuOpen` true)
        (bind _returnvalue (`|CreateWidget` "/Game/Widgets/WBP_PauseMenu.WBP_PauseMenu_C" (`GameplayStatics.GetPlayerController` 0)))
        (bind _output_get (set `self.PauseMenuREF` _returnvalue))
        (`UserWidget.AddToViewport` _output_get 0)
        (`WidgetBlueprintLibrary.SetInputMode_UIOnlyEx` self (`self.PauseMenuREF`))
        (set `self.bShowMouseCursor` true)
        (`GameplayStatics.SetGamePaused` true)))))

(event `Key|P`
  (params (Key :type "Key Structure"))
  (:`Pressed`
    (if (`self.IsPauseMenuOpen`)
      (set `self.IsPauseMenuOpen` false)
      (`Widget.RemoveFromParent` (`self.PauseMenuREF`))
      (set `self.PauseMenuREF` null)
      (`WidgetBlueprintLibrary.SetInputMode_GameOnly` self)
      (set `self.bShowMouseCursor` false)
      (`GameplayStatics.SetGamePaused` false)
      (else
        (set `self.IsPauseMenuOpen` true)
        (bind _returnvalue (`|CreateWidget` "/Game/Widgets/WBP_PauseMenu.WBP_PauseMenu_C" (`GameplayStatics.GetPlayerController` 0)))
        (bind _output_get (set `self.PauseMenuREF` _returnvalue))
        (`UserWidget.AddToViewport` _output_get 0)
        (`WidgetBlueprintLibrary.SetInputMode_UIOnlyEx` self (`self.PauseMenuREF`))
        (set `self.bShowMouseCursor` true)
        (`GameplayStatics.SetGamePaused` true)))))

(fn `LineTrace`
  (params (Length :type "Float (double-precision)") (DrawDebugType :type "EDrawDebugTrace Enum" :default "None"))
  (returns (HItActor :type "Actor Object Reference"))
  (bind _asl1_character (cast `/Game/Blueprints/Level1/L1_Character` (`GameplayStatics.GetPlayerCharacter` 0)))
  (bind _camera (`/Game/Blueprints/Level1/L1_Character.Camera` _asl1_character))
  (bind _returnvalue (`SceneComponent.K2_GetComponentLocation` _camera))
  (bind _outhit (`KismetSystemLibrary.LineTraceSingle` :`Start` _returnvalue :`End` (+ _returnvalue (* (`SceneComponent.GetForwardVector` _camera) Length)) :`TraceChannel` "TraceTypeQuery1" :`DrawDebugType` DrawDebugType))
  (return (`.HitActor` (`GameplayStatics.BreakHitResult` _outhit))))

(fn `UserConstructionScript`)