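; Movement component that handles walk speed and stamina-gated sprinting for a character.
; Initialize stores the character reference and applies walk speed to both standing and crouched movement.
; StartSprint raises max walk speed when stamina exceeds the minimum, then requests SprintTimer by function name to drain clamped stamina.
; No stop-sprint or stamina regeneration logic is present.
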(event `StartSprint`
  (if (> (`self.CurrentStamina`) (`self.MinStamina`))
    (`self.Set Player Max Speed` (`self.SprintSpeed`))
    (`KismetSystemLibrary.K2_SetTimer` null "SprintTimer")))

(event `SprintTimer`
  (set `self.CurrentStamina` (`KismetMathLibrary.FClamp` (- (`self.CurrentStamina`) 1.0))))

(fn `Initialize`
  (params (Character :type "Character Object Reference"))
  (set `self.PlayerRef` Character)
  (set `CharacterMovementComponent.MaxWalkSpeed` (`self.WalkSpeed`) (`Character.CharacterMovement` (`self.PlayerRef`)))
  (set `CharacterMovementComponent.MaxWalkSpeedCrouched` (`self.WalkSpeed`) (`Character.CharacterMovement` (`self.PlayerRef`))))

(fn `Set Player Max Speed`
  (params (`Max Walk Speed` :type "Float (single-precision)"))
  (set `CharacterMovementComponent.MaxWalkSpeed` `Max Walk Speed` (`Character.CharacterMovement` (`self.PlayerRef`))))