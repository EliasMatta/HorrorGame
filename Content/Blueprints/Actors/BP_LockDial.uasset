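; BP_LockDial is a single rotating number dial of a lock, with up and down arrow widgets and a random starting digit.
; A timeline, played forward or in reverse, animates each 36-degree step while a flag blocks overlapping turns.
; On finish it wraps the rotation, derives the 0–9 digit from the angle and tells the owning lock to check after every turn.
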(event `self.ReceiveBeginPlay`
  (`/Game/Widgets/WBP_Arrow.Initialize` (cast `/Game/Widgets/WBP_Arrow` (`WidgetComponent.GetUserWidgetObject` (`self.UpArrow`)) :!pure true) self true)
  (`/Game/Widgets/WBP_Arrow.Initialize` (cast `/Game/Widgets/WBP_Arrow` (`WidgetComponent.GetUserWidgetObject` (`self.DownArrow`)) :!pure true) self false)
  (`self.Set Random Number`))

(event `FindNumber`
  (set `self.Number` (`KismetMathLibrary.Abs_Int` (`KismetMathLibrary.FTrunc` (/ (`self.DialRotation`) -36.0)))))

(event `RotateDIal`
  (bind _dialrotation (`self.DialRotation`))
  (if (`self.canRotate`)
    (set `self.canRotate` false)
    (bind (_direction _alpha) (`Timeline|RotateDialTL` :!via `PlayFromStart` :!label _label)
      (:`Update`
        (bind _returnvalue (- (`self.DialRotation`) (select `ETimelineDirection` _direction :`Forward` (`KismetMathLibrary.Lerp` 0.0 36.0 _alpha) :`Backward` (`KismetMathLibrary.Lerp` -36.0 0.0 _alpha))))
        (`SceneComponent.K2_SetRelativeRotation` (`self.LockDial`) (`KismetMathLibrary.MakeRotator` 0.0 _returnvalue) false false))
      (:`Finished`
        (set `self.DialRotation` _returnvalue)
        (if (<= _dialrotation -360.0)
          (set `self.DialRotation` 0.0)
          (`SceneComponent.K2_SetRelativeRotation` :`self` (`self.LockDial`))
          (elif (> _dialrotation 0.0)
            (bind _output_get (set `self.DialRotation` (`KismetMathLibrary.MapRangeClamped` (`self.DialRotation`) 0.0 360.0 -360.0)))
            (`SceneComponent.K2_SetRelativeRotation` (`self.LockDial`) (`KismetMathLibrary.MakeRotator` 0.0 _output_get) false false)))
        (`self.FindNumber`)
        (`/Game/Blueprints/Actors/BP_Lock.CheckEveryTurn` (`self.BPLockRef`))
        (set `self.canRotate` true)))))

(event `RotateDialBackWards`
  (if (`self.canRotate`)
    (set `self.canRotate` false)
    (goto _label :!via `ReverseFromEnd`)))

(fn `Set Random Number`
  (locals (localRoatation :type Integer))
  (set `local.localRoatation` (* (`KismetMathLibrary.RandomIntegerInRange` 0 9) -36))
  (`SceneComponent.K2_SetRelativeRotation` (`self.LockDial`) (`KismetMathLibrary.MakeRotator` 0.0 (`KismetMathLibrary.Conv_IntToDouble` (`local.localRoatation`))) false false)
  (set `self.DialRotation` (`KismetMathLibrary.Conv_IntToDouble` (`local.localRoatation`)))
  (`self.FindNumber`))

(fn `UserConstructionScript`)