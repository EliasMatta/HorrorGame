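; Interactable combination safe: Interact hides the player, disables movement, switches to the safe camera and enables input.
; Q and E drive timelines that turn the knob and count update ticks, with sound cues at each side's target count.
; Hitting both targets, in either order, unlocks the safe and disables Box collision.
; Space then swings the door open via timeline and restores player view, visibility and walking.
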(event `Key|Q`
  (params (Key :type "Key Structure"))
  (:`Pressed`
    (bind (_direction _leftspin) (`Timeline|LeftSpin` :`NewTime` 2.0 :!via `SetNewTime`)
      (:`Update`
        (`SceneComponent.K2_AddLocalRotation` (`self.SafeKnob`) (`KismetMathLibrary.MakeRotator` 0.0 _leftspin) false false)
        (bind _output_get (set `self.LeftSpinValue` (+ (`self.LeftSpinValue`) 1)))
        (`/Engine/EditorBlueprintResources/StandardMacros.CompareInt` _output_get 14
          (:`==`
            (bind _output_get_2 (set `self.PreUnlockerLeft` 14))
            (`GameplayStatics.PlaySound2D` "/Game/Sounds/SafeSoundOpen.SafeSoundOpen" 3.0 2.0 0.0 null null)
            (`/Engine/EditorBlueprintResources/StandardMacros.CompareInt` (+ _output_get_2 (stale `Key|E` _output_get_2)) 35 :!label _label
              (:`==`
                (`GameplayStatics.PlaySound2D` "/Game/Sounds/SafeSoundOpen.SafeSoundOpen" 4.0 1.0 0.0 null null)
                (`KismetSystemLibrary.Delay` 0.5)
                (`GameplayStatics.PlaySound2D` "/Game/Sounds/SafeSoundOpen.SafeSoundOpen" 4.0 1.0 0.0 null null)
                (set `self.SafeUnlocked` true)
                (`PrimitiveComponent.SetCollisionEnabled` (`self.Box`) "NoCollision")))))))))

(event `Key|E`
  (params (Key :type "Key Structure"))
  (:`Pressed`
    (bind (_direction _rightspin) (`Timeline|RIghtSpin` :!via `Reverse`)
      (:`Update`
        (`SceneComponent.K2_AddLocalRotation` (`self.SafeKnob`) (`KismetMathLibrary.MakeRotator` 0.0 _rightspin) false false)
        (bind _output_get (set `self.RightSpinValue` (+ (`self.RightSpinValue`) 1)))
        (`/Engine/EditorBlueprintResources/StandardMacros.CompareInt` _output_get 21
          (:`==`
            (bind _output_get_2 (set `self.PreUnlockerRight` 21))
            (`GameplayStatics.PlaySound2D` "/Game/Sounds/SafeSoundOpen.SafeSoundOpen" 3.0 3.0 0.0 null null)
            (goto _label)))))))

(event `Key|SpaceBar`
  (params (Key :type "Key Structure"))
  (:`Pressed`
    (if (`self.SafeUnlocked`)
      (bind (_direction _safedooropener) (`Timeline|SafeDoorOpen`)
        (:`Update`
          (`SceneComponent.K2_AddRelativeRotation` (`self.SafeDoor`) (`KismetMathLibrary.MakeRotator` 0.0 0.0 _safedooropener) false false)
          (bind _asl1_character (cast `/Game/Blueprints/Level1/L1_Character` (`GameplayStatics.GetPlayerCharacter` 0)))
          (`PlayerController.SetViewTargetWithBlend` (`GameplayStatics.GetPlayerController` 0) (`ActorComponent.GetOwner` (`/Game/Blueprints/Level1/L1_Character.Camera` _asl1_character)) 0.4 "VTBlend_Linear" 0.0 false)
          (`SceneComponent.SetVisibility` (`Character.Mesh` _asl1_character) true false)
          (`CharacterMovementComponent.SetMovementMode` (`Character.CharacterMovement` _asl1_character) "MOVE_Walking" 0)
          (`self.DisableInput` (`GameplayStatics.GetPlayerController` 0))
          (`SceneComponent.SetVisibility` (`self.Pointer`) false false))))))

(event `/Game/Blueprints/Interfaces/BPI_Interaction.Interact`
  (bind _asl1_character (cast `/Game/Blueprints/Level1/L1_Character` (`GameplayStatics.GetPlayerCharacter` 0)))
  (`SceneComponent.SetVisibility` (`Character.Mesh` _asl1_character) false false)
  (`PlayerController.SetViewTargetWithBlend` (`GameplayStatics.GetPlayerController` 0) (`ActorComponent.GetOwner` (`self.CameraSafeView`)) 0.0 "VTBlend_Linear" 0.0 false)
  (`self.EnableInput` (`GameplayStatics.GetPlayerController` 0))
  (`CharacterMovementComponent.DisableMovement` (`Character.CharacterMovement` (`GameplayStatics.GetPlayerCharacter` 0))))

(fn `UserConstructionScript`)