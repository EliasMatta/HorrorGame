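; Keypad actor that unlocks a linked BPDoor when the player enters the correct passcode.
; Overlapping its collision box registers it with L1_Character; interacting blends to the keypad camera, locks movement and shows the cursor.
; Child-actor Keypad_Button digits edit a text render, capped at four characters, which is compared to KeypadCode on confirm.
; Success restores control, removes the collision box and opens the door; failure shows red feedback and re-arms entry.
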(event `self.CollisionBox.OnComponentBeginOverlap`
  (params (OverlappedComponent :type "PrimitiveComponent Object Reference") (OtherActor :type "Actor Object Reference") (OtherComp :type "PrimitiveComponent Object Reference") (OtherBodyIndex :type Integer) (bFromSweep :type Boolean) (SweepResult :type "HitResult Structure (by ref)"))
  (if (== OtherActor (`GameplayStatics.GetPlayerPawn` 0))
    (bind _asl1_character (cast `/Game/Blueprints/Level1/L1_Character` OtherActor))
    (set `/Game/Blueprints/Level1/L1_Character.KeypadInteract` self _asl1_character)
    (set `self.PlayerREf` _asl1_character)))

(event `self.CollisionBox.OnComponentEndOverlap`
  (params (OverlappedComponent :type "PrimitiveComponent Object Reference") (OtherActor :type "Actor Object Reference") (OtherComp :type "PrimitiveComponent Object Reference") (OtherBodyIndex :type Integer))
  (if (== OtherActor (`GameplayStatics.GetPlayerPawn` 0))
    (bind _asl1_character (cast `/Game/Blueprints/Level1/L1_Character` OtherActor))
    (set `/Game/Blueprints/Level1/L1_Character.KeypadInteract` null _asl1_character)
    (set `self.PlayerREf` null)))

(event `OnInteracted`
  (bind _returnvalue (`GameplayStatics.GetPlayerController` 0))
  (bind _returnvalue_2 (`GameplayStatics.GetPlayerController` 0))
  (bind _enteredcodetext (`self.EnteredCodeText`))
  (bind _asl1_character (cast `/Game/Blueprints/Level1/L1_Character` (`GameplayStatics.GetPlayerCharacter` 0)))
  (set `/Game/Blueprints/Level1/L1_Character.canOpenInventory` false _asl1_character)
  (`CharacterMovementComponent.DisableMovement` (`Character.CharacterMovement` (`GameplayStatics.GetPlayerCharacter` 0)))
  (`self.DisableInput` _returnvalue null)
  (`Controller.SetIgnoreLookInput` _returnvalue false)
  (`PlayerController.SetViewTargetWithBlend` (`GameplayStatics.GetPlayerController` 0) (`ActorComponent.GetOwner` (`self.Camera`)) 0.4 "VTBlend_Linear" 0.0 false)
  (bind _output_get (set `PlayerController.bShowMouseCursor` true _returnvalue_2 :!label _label))
  (bind _output_get_2 (set `PlayerController.bEnableClickEvents` _output_get _returnvalue_2))
  (set `PlayerController.bEnableMouseOverEvents` _output_get_2 _returnvalue_2)
  (`TextRenderComponent.K2_SetText` _enteredcodetext (`KismetSystemLibrary.MakeLiteralText` (`KismetTextLibrary.Conv_StringToText` (`KismetStringLibrary.GetSubstring` "...." 0 (`KismetStringLibrary.Len` (`self.Keypad Code`))))))
  (`TextRenderComponent.SetTextRenderColor` _enteredcodetext (make `Color` 255 255 255 255))
  (bind _output_get_3 (set `self.ButtonsArray` (`|MakeArray` (`self.Keypad_Button1`) (`self.Keypad_Button2`) (`self.Keypad_Button3`) (`self.Keypad_Button4`) (`self.Keypad_Button5`) (`self.Keypad_Button6`) (`self.Keypad_Button7`) (`self.Keypad_Button8`) (`self.Keypad_Button9`) (`self.Keypad_Button_Backspace`) (`self.Keypad_Button0`) (`self.Keypad_Button_Confirm`))))
  (for _array_element _output_get_3
    (bind _askeypad_button (cast `/Game/Blueprints/Actors/Keypad/Keypad_Button` (`ChildActorComponent.ChildActor` _array_element)))
    (set `/Game/Blueprints/Actors/Keypad/Keypad_Button.KeypadActorREF` self _askeypad_button)))

(event `Initiate`
  (goto _label))

(event `ButtonClicked`
  (params (Value :type Text) (Confirmed :type Boolean) (BackSpace :type Boolean))
  (bind _enteredcodetext (`self.EnteredCodeText`))
  (bind _returnvalue (`KismetStringLibrary.Concat_StrStr` (`KismetTextLibrary.Conv_TextToString` (`TextRenderComponent.Text` (`self.EnteredCodeText`))) (`KismetTextLibrary.Conv_TextToString` Value)))
  (if Confirmed
    (`self.OnConfirmed`)
    (elif BackSpace
      (`self.BackSpace`)
      (elif (`self.Can Enter`)
        (`GameplayStatics.PlaySound2D` "/Game/HorrorEngine/Audio/Elecronic/LockPanelButton.LockPanelButton" 1.0 1.0 0.0 null null)
        (`TextRenderComponent.K2_SetText` _enteredcodetext (`KismetTextLibrary.Conv_StringToText` (`KismetStringLibrary.Replace` (`KismetTextLibrary.Conv_TextToString` (`TextRenderComponent.Text` (`self.EnteredCodeText`))) (`KismetStringLibrary.GetSubstring` "...." 0 (`KismetStringLibrary.Len` (`self.Keypad Code`))))))
        (if (<= (`KismetStringLibrary.Len` _returnvalue) 4)
          (`TextRenderComponent.K2_SetText` _enteredcodetext (`KismetTextLibrary.Conv_StringToText` _returnvalue))
          (`TextRenderComponent.SetTextRenderColor` (`self.EnteredCodeText`) (make `Color` 255 255 255 255)))))))

(event `BackSpace`
  (bind _enteredcodetext (`self.EnteredCodeText`))
  (bind _returnvalue (`KismetTextLibrary.Conv_TextToString` (`TextRenderComponent.Text` _enteredcodetext)))
  (`TextRenderComponent.K2_SetText` _enteredcodetext (`KismetTextLibrary.Conv_StringToText` (`KismetStringLibrary.GetSubstring` _returnvalue 0 (- (`KismetStringLibrary.Len` _returnvalue) 1)))))

(event `OnConfirmed`
  (bind _returnvalue (`GameplayStatics.GetPlayerController` 0))
  (bind _returnvalue_2 (`GameplayStatics.GetPlayerController` 0))
  (bind _returnvalue_3 (`GameplayStatics.GetPlayerController` 0))
  (bind _enteredcodetext (`self.EnteredCodeText`))
  (bind _enteredcodetext_2 (`self.EnteredCodeText`))
  (bind _bp_door (`self.BP_Door`))
  (bind _asl1_character (cast `/Game/Blueprints/Level1/L1_Character` (`GameplayStatics.GetPlayerCharacter` 0) :!pure true))
  (if true
    (if (`KismetStringLibrary.EqualEqual_StrStr` (`self.Keypad Code`) (`KismetTextLibrary.Conv_TextToString` (`TextRenderComponent.Text` (`self.EnteredCodeText`))))
      (`|ExecutionSequence`
        (:`then_0`
          (`TextRenderComponent.K2_SetText` _enteredcodetext_2 "Correct Passcode!")
          (`TextRenderComponent.SetTextRenderColor` _enteredcodetext_2 (make `Color` 0 255 0 255))
          (`PrimitiveComponent.SetMaterial` (`self.Keypad`) 2 "/Game/Blueprints/Actors/Keypad/M_GreenGlow.M_GreenGlow")
          (`KismetSystemLibrary.RetriggerableDelay` 0.1)
          (bind _output_get (set `PlayerController.bShowMouseCursor` false _returnvalue_3))
          (bind _output_get_2 (set `PlayerController.bEnableMouseOverEvents` _output_get _returnvalue_3))
          (set `PlayerController.bEnableClickEvents` _output_get_2 _returnvalue_3)
          (for _array_element (`self.ButtonsArray`)
            (bind _askeypad_button (cast `/Game/Blueprints/Actors/Keypad/Keypad_Button` (`ChildActorComponent.ChildActor` _array_element)))
            (`/Game/Blueprints/Actors/Keypad/Keypad_Button.ResetButton` _askeypad_button))
          (`CharacterMovementComponent.SetMovementMode` (`Character.CharacterMovement` _asl1_character) "MOVE_Walking" 0)
          (`PlayerController.SetViewTargetWithBlend` (`GameplayStatics.GetPlayerController` 0) (`ActorComponent.GetOwner` (`/Game/Blueprints/Level1/L1_Character.Camera` _asl1_character)) 0.4 "VTBlend_Linear" 0.0 false)
          (`TextRenderComponent.K2_SetText` (`self.EnteredCodeText`) "")
          (`self.EnableInput` _returnvalue null)
          (`Controller.SetIgnoreLookInput` _returnvalue true)
          (set `PlayerController.bShowMouseCursor` false _returnvalue)
          (`WidgetBlueprintLibrary.SetInputMode_GameOnly` (`GameplayStatics.GetPlayerController` 0))
          (bind _asl1_character_2 (cast `/Game/Blueprints/Level1/L1_Character` (`GameplayStatics.GetPlayerCharacter` 0)))
          (set `/Game/Blueprints/Level1/L1_Character.canOpenInventory` true _asl1_character_2)
          (`ActorComponent.K2_DestroyComponent` (`self.CollisionBox`))
          (set `DoorInteract.bIsInteracting` true _bp_door)
          (`DoorInteract.Interact` _bp_door))
        (:`then_1`
          (set `self.Can Enter` false)
          (`GameplayStatics.PlaySound2D` "/Game/HorrorEngine/Audio/Elecronic/KeyCardOpen.KeyCardOpen" 1.0 1.0 0.0 null null)))
      (else
        (`|ExecutionSequence`
          (:`then_0`
            (`TextRenderComponent.K2_SetText` _enteredcodetext "Wrong  Passcode!")
            (`TextRenderComponent.SetTextRenderColor` _enteredcodetext (make `Color` 0 0 255 255))
            (`PrimitiveComponent.SetMaterial` (`self.Keypad`) 2 "/Game/Blueprints/Actors/Keypad/M_RedGlow.M_RedGlow")
            (`KismetSystemLibrary.RetriggerableDelay` 0.1)
            (bind _output_get_3 (set `PlayerController.bEnableMouseOverEvents` false _returnvalue_2))
            (set `PlayerController.bEnableClickEvents` _output_get_3 _returnvalue_2)
            (for _array_element_2 (`self.ButtonsArray`)
              (bind _askeypad_button_2 (cast `/Game/Blueprints/Actors/Keypad/Keypad_Button` (`ChildActorComponent.ChildActor` _array_element_2)))
              (`/Game/Blueprints/Actors/Keypad/Keypad_Button.ResetButton` _askeypad_button_2))
            (`self.Initiate`)
            (set `self.Can Enter` true))
          (:`then_1`
            (set `self.Can Enter` false)
            (`GameplayStatics.PlaySound2D` "/Game/HorrorEngine/Audio/Elecronic/KeyCardDenied.KeyCardDenied" 1.0 1.0 0.0 null null)))))))

(fn `UserConstructionScript`)