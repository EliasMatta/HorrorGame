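; Collectible paper pickup that counts toward unlocking an exit door in the level.
; BeginPlay registers it with L1_Gamemode's pickup amount and gathers all exit doors.
; Interact makes it grabbable and shows the HUD paper counter; Tick then polls the gamemode's PlayerInteract flag to play a sound, destroy the paper and increment the collected count.
; The fifth pickup sets AllPapersCollected on one randomly chosen BP_ExitDoor.
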(event `self.ReceiveBeginPlay`
  (bind _outactors (`GameplayStatics.GetAllActorsOfClass` "/Game/Blueprints/Actors/Interaction/BP_ExitDoor.BP_ExitDoor_C"))
  (bind _asl1_gamemode (cast `/Game/Blueprints/Level1/L1_Gamemode` (`GameplayStatics.GetGameMode`)))
  (set `/Game/Blueprints/Level1/L1_Gamemode.PickupAmount` (+ (`/Game/Blueprints/Level1/L1_Gamemode.PickupAmount` _asl1_gamemode) 1) _asl1_gamemode))

(event `/Game/Blueprints/Interfaces/BPI_Interaction.Interact`
  (set `self.Grabbable` true)
  (bind _asl1_character (cast `/Game/Blueprints/Level1/L1_Character` (`GameplayStatics.GetPlayerCharacter` 0)))
  (`/Game/Widgets/WBP_MainHUD.ShowPaperCounter` (`/Game/Blueprints/Level1/L1_Character.MAINHUD` _asl1_character)))

(event `self.ReceiveTick`
  (params (DeltaSeconds :type "Float (single-precision)"))
  (if (`self.Grabbable`)
    (bind _asl1_gamemode (cast `/Game/Blueprints/Level1/L1_Gamemode` (`GameplayStatics.GetGameMode`)))
    (if (`/Game/Blueprints/Level1/L1_Gamemode.PlayerInteract` _asl1_gamemode)
      (`/Engine/EditorBlueprintResources/StandardMacros.DoOnce` false
        (:`Completed`
          (`GameplayStatics.PlaySound2D` "/Game/HorrorEngine/Audio/Paper/Paper01.Paper01" 4.0 1.0 0.0 null null)
          (`self.K2_DestroyActor`)
          (bind _output_get (set `/Game/Blueprints/Level1/L1_Gamemode.Pickups` (`KismetMathLibrary.Clamp` (+ (`/Game/Blueprints/Level1/L1_Gamemode.Pickups` _asl1_gamemode) 1) 0 5) _asl1_gamemode))
          (if (== _output_get 5)
            (set `DoorInteract.bAllPapersCollected` true (`|GetArrayItem` (stale `self.ReceiveBeginPlay` _outactors) (`KismetMathLibrary.RandomIntegerInRange` 0 (- (`KismetArrayLibrary.Array_Length` (stale `self.ReceiveBeginPlay` _outactors)) 1))))))))))

(fn `UserConstructionScript`)