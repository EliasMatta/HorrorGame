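; An interactable light switch actor that turns a referenced Light on and off.
; Each Interact event alternates through a FlipFlop, playing a click sound at the switch, setting the light's visibility and playing or reversing a timeline that tilts the switch's pitch.
; The toggle does not read the light's current state, so the first interaction always turns it on; an unconnected branch with a validity and visibility check never runs.
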(event `/Game/Blueprints/Interfaces/BPI_Interaction.Interact`
  (`/Engine/EditorBlueprintResources/StandardMacros.FlipFlop`
    (:`A`
      (`GameplayStatics.PlaySoundAtLocation` "/Engine/VREditor/Sounds/UI/Flashlight_Switch.Flashlight_Switch" (`SceneComponent.K2_GetComponentLocation` (`self.LightSwitch`)) (struct) 13.0 1.0 0.0 null null null null)
      (`SceneComponent.SetVisibility` (`Light.LightComponent` (`self.Light`)) true false)
      (bind (_direction _lightswitchalpha) (`Timeline|LightSwitch_TL` :!label _label)
        (:`Update`
          (`SceneComponent.K2_SetRelativeRotation` (`self.LightSwitch`) (`KismetMathLibrary.MakeRotator` 0.0 (`KismetMathLibrary.Lerp` 9.0 -9.0 _lightswitchalpha)) false false))))
    (:`B`
      (`GameplayStatics.PlaySoundAtLocation` "/Engine/VREditor/Sounds/UI/Flashlight_Switch.Flashlight_Switch" (`SceneComponent.K2_GetComponentLocation` (`self.LightSwitch`)) (struct) 12.0 -10.0 0.0 null null null null)
      (`SceneComponent.SetVisibility` (`Light.LightComponent` (`self.Light`)) false false)
      (goto _label :!via `Reverse`))))

(fn `UserConstructionScript`)