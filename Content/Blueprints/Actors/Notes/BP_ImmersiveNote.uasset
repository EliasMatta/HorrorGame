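; Note actor that opens a note examination widget on screen.
; On BeginPlay it caches the first BP_NotesExamination found in the level.
; Pressing Backspace creates a new WBP_NoteExamination with that reference, passes itself to UpdateWidget and adds it to the viewport.
; The construction script's node for setting NoteText is disconnected, so it never runs.
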(event `self.ReceiveBeginPlay`
  (bind _outactors (`GameplayStatics.GetAllActorsOfClass` "/Game/Blueprints/Actors/Notes/BP_NotesExamination.BP_NotesExamination_C"))
  (set `self.BPNoteExaminationRef` (`|GetArrayItem` _outactors)))

(event `Key|BackSpace`
  (params (Key :type "Key Structure"))
  (:`Pressed`
    (bind _returnvalue (`|CreateWidget` "/Game/Widgets/WBP_NoteExamination.WBP_NoteExamination_C" null null (`self.BPNoteExaminationRef`)))
    (`/Game/Widgets/WBP_NoteExamination.UpdateWidget` _returnvalue self)
    (`UserWidget.AddToViewport` _returnvalue 0)))

(fn `UserConstructionScript`)