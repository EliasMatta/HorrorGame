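; Key inventory item that, when used, tries to interact with doors in the level and reports whether the use worked.
; UseItem loops over every DoorInteract actor and calls TryInteract on each.
; The first successful door that requires a key sets UseItemSucess, plays the door-open sound at world origin and ends the loop; other outcomes leave the flag false.
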(event `self.UseItem`
  (bind _outactors (`GameplayStatics.GetAllActorsOfClass` "/Script/HorrorGame.DoorInteract"))
  (for _array_element _outactors
    (bind _returnvalue (`DoorInteract.TryInteract` _array_element))
    (if _returnvalue
      (if (`DoorInteract.bRequiresKey` _array_element)
        (set `self.UseItemSucess` true)
        (`GameplayStatics.PlaySoundAtLocation` "/Game/Sounds/DoorOpen.DoorOpen" (0.0 0.0 0.0) (struct) 1.0 1.0 0.0 null null null null)
        (break)
        (else
          (set `self.UseItemSucess` false)))))
  (if (not _returnvalue)
    (set `self.UseItemSucess` false)))

(event `self.ReceiveBeginPlay`)

(fn `UserConstructionScript`
  (`parent.UserConstructionScript`))