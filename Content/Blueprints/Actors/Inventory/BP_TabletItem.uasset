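; BP_TabletItem is an inventory item that opens a camera view interface when used.
; Its UseItem event collapses the player's inventory menu, then creates a WBP_MainViewCams widget, stores it and adds it to the viewport.
; Each use creates a new widget instance, and the other events and construction script add no logic of their own.
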(event `self.UseItem`
  (`Widget.SetVisibility` (`/Game/Blueprints/Level1/L1_Character.InventoryMenu` (`self.PlayerRef`)) "Collapsed")
  (bind _returnvalue (`|CreateWidget` "/Game/Blueprints/Actors/SecurityCamera/WBP_MainViewCams.WBP_MainViewCams_C" null null))
  (bind _output_get (set `self.MainViewCams` _returnvalue))
  (`UserWidget.AddToViewport` _output_get 0))

(fn `UserConstructionScript`
  (`parent.UserConstructionScript`))