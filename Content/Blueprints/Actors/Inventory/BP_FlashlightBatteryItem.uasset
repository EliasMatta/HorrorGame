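; Inventory item that recharges the player's flashlight when used.
; UseItem adds BatteryAmount through the FlashlightComponent on PlayerRef, but only if the current battery level is below its maximum.
; It sets the UseItemSucess flag to report whether the battery was applied.
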(event `self.UseItem`
  (bind _flashlightcomponent (`/Game/Blueprints/Level1/L1_Character.FlashlightComponent` (`self.PlayerRef`)))
  (if (< (`FlashlightComponent.CurrentBatteryLevel` _flashlightcomponent) (`FlashlightComponent.MaxBatteryLevel` _flashlightcomponent))
    (`FlashlightComponent.AddBatteryLife` _flashlightcomponent (`self.BatteryAmount`))
    (set `self.UseItemSucess` true)
    (else
      (set `self.UseItemSucess` false))))

(fn `UserConstructionScript`
  (`parent.UserConstructionScript`))