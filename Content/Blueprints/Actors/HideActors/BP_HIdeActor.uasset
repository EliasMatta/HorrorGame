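; Hiding spot actor that lets the player enter and leave concealment through Interact, toggled by the character's IsHiding flag.
; Entering notifies one zombie, big zombie and monster AI controller, then disables mesh collision, movement and inventory.
; A looping timer glides the player between hiding and exit points, aligning view to the actor's rotation.
; On finishing, it flips IsHiding; exiting also notifies those controllers and restores player control.
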(event `self.ReceiveBeginPlay`
  (bind _asl1_character (cast `/Game/Blueprints/Level1/L1_Character` (`GameplayStatics.GetPlayerCharacter` 0)))
  (set `self.PlayerRef` _asl1_character))

(event `/Game/Blueprints/Interfaces/BPI_Interaction.Interact`
  (bind _playerref (`self.PlayerRef`))
  (if (`/Game/Blueprints/Level1/L1_Character.isHiding` (`self.PlayerRef`))
    (bind _returnvalue (`KismetSystemLibrary.K2_SetTimerDelegate` (delegate `MoveCharacter`) (`GameplayStatics.GetWorldDeltaSeconds`) true))
    (else
      (bind _asaic_big_zombie (castclass `/Game/AI/BigZombieAI/AIC_BigZombie` "/Game/AI/BigZombieAI/AIC_BigZombie.AIC_BigZombie_C"))
      (bind _returnvalue_2 (`GameplayStatics.GetActorOfClass` _asaic_big_zombie))
      (message `/Game/Blueprints/Interfaces/BPI_PlayerHiding.DidEnemySee` _returnvalue_2 self)
      (bind _asaic_zombie (castclass `/Game/AI/ZombieAI/AIC_Zombie` "/Game/AI/ZombieAI/AIC_Zombie.AIC_Zombie_C"))
      (bind _returnvalue_3 (`GameplayStatics.GetActorOfClass` _asaic_zombie))
      (message `/Game/Blueprints/Interfaces/BPI_PlayerHiding.DidEnemySee` _returnvalue_3 self)
      (bind _asaic_monster (castclass `/Game/AI/MonsterAI/AIC_Monster` "/Game/AI/MonsterAI/AIC_Monster.AIC_Monster_C"))
      (bind _returnvalue_4 (`GameplayStatics.GetActorOfClass` _asaic_monster))
      (message `/Game/Blueprints/Interfaces/BPI_PlayerHiding.DidEnemySee` _returnvalue_4 self)
      (`PrimitiveComponent.SetCollisionEnabled` (`Character.Mesh` _playerref) "NoCollision")
      (`CharacterMovementComponent.DisableMovement` (`Character.CharacterMovement` _playerref))
      (set `/Game/Blueprints/Level1/L1_Character.canOpenInventory` false (`self.PlayerRef`))
      (bind _returnvalue_5 (`KismetSystemLibrary.K2_SetTimerDelegate` (delegate `MoveCharacter`) (`GameplayStatics.GetWorldDeltaSeconds`) true)))))

(event `MoveCharacter`
  (bind _returnvalue (`self.K2_GetActorRotation`))
  (bind _playerref (`self.PlayerRef`))
  (`self.K2_SetActorTransform` _playerref (`KismetMathLibrary.MakeTransform` (`KismetMathLibrary.VInterpTo_Constant` (`self.K2_GetActorLocation` _playerref) (`SceneComponent.K2_GetComponentLocation` (select `bool` (`/Game/Blueprints/Level1/L1_Character.isHiding` (`self.PlayerRef`)) :`false` (`self.HidingPosition`) :`true` (`self.ExitPosition`) :!type "SceneComponent Object Reference")) (`GameplayStatics.GetWorldDeltaSeconds`) 1000.0) _returnvalue) false false)
  (`Controller.SetControlRotation` (`Pawn.GetLocalViewingPlayerController` _playerref) _returnvalue)
  (if (== (`self.K2_GetActorLocation` (`self.PlayerRef`)) (`SceneComponent.K2_GetComponentLocation` (select `bool` (`/Game/Blueprints/Level1/L1_Character.isHiding` (`self.PlayerRef`)) :`false` (`self.HidingPosition`) :`true` (`self.ExitPosition`) :!type "SceneComponent Object Reference")) :`ErrorTolerance` 0.01)
    (`KismetSystemLibrary.K2_ClearAndInvalidateTimerHandle` (stale `/Game/Blueprints/Interfaces/BPI_Interaction.Interact` _returnvalue_5))
    (`KismetSystemLibrary.K2_ClearAndInvalidateTimerHandle` (stale `/Game/Blueprints/Interfaces/BPI_Interaction.Interact` _returnvalue))
    (`self.FinishedMoving`)))

(event `FinishedMoving`
  (bind _playerref (`self.PlayerRef`))
  (bind _playerref_2 (`self.PlayerRef`))
  (`self.FinishedMovingED`)
  (if (`/Game/Blueprints/Level1/L1_Character.isHiding` _playerref)
    (set `/Game/Blueprints/Level1/L1_Character.isHiding` false _playerref)
    (bind _asaic_big_zombie (castclass `/Game/AI/BigZombieAI/AIC_BigZombie` "/Game/AI/BigZombieAI/AIC_BigZombie.AIC_BigZombie_C"))
    (bind _returnvalue (`GameplayStatics.GetActorOfClass` _asaic_big_zombie))
    (message `/Game/Blueprints/Interfaces/BPI_PlayerHiding.LeftHidingSpot` _returnvalue)
    (bind _asaic_zombie (castclass `/Game/AI/ZombieAI/AIC_Zombie` "/Game/AI/ZombieAI/AIC_Zombie.AIC_Zombie_C"))
    (bind _returnvalue_2 (`GameplayStatics.GetActorOfClass` _asaic_zombie))
    (message `/Game/Blueprints/Interfaces/BPI_PlayerHiding.LeftHidingSpot` _returnvalue_2)
    (bind _asaic_monster (castclass `/Game/AI/MonsterAI/AIC_Monster` "/Game/AI/MonsterAI/AIC_Monster.AIC_Monster_C"))
    (bind _returnvalue_3 (`GameplayStatics.GetActorOfClass` _asaic_monster))
    (message `/Game/Blueprints/Interfaces/BPI_PlayerHiding.LeftHidingSpot` _returnvalue_3)
    (`self.SetActorEnableCollision` _playerref_2 true)
    (`CharacterMovementComponent.SetMovementMode` (`Character.CharacterMovement` _playerref_2) "MOVE_Walking" 0)
    (set `/Game/Blueprints/Level1/L1_Character.canOpenInventory` true (`self.PlayerRef`))
    (else
      (set `/Game/Blueprints/Level1/L1_Character.isHiding` true _playerref))))

(event `PlayerFound`)

(fn `UserConstructionScript`)