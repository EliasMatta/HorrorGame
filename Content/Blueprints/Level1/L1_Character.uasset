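; Level 1 first-person player character handling interaction, inventory, flashlight, puzzle rotation and enemy catches.
; Initialize creates crosshair, HUD and inventory widgets; ToggleInventory only opens the menu, locking movement and look.
; Tick line-traces from the camera to show the crosshair over interactables, while Q/E trace to send rotate messages to puzzles.
; Interact sets a gamemode flag and triggers the keypad; CaughtByEnemies removes health and calls the enemy's KillPlayer.
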(event `self.ReceiveBeginPlay`
  (`self.Initialize`))

(event `EnhancedInput|/Game/Inputs/InputActions/IA_Inventory`
  (params (ActionValue :type Boolean) (ElapsedSeconds :type "Float (double-precision)") (TriggeredSeconds :type "Float (double-precision)") (InputAction :type "InputAction Object Reference" :default "/Game/Inputs/InputActions/IA_Inventory.IA_Inventory"))
  (:`Started`
    (`self.ToggleInventory`)))

(event `EnhancedInput|/Game/Inputs/InputActions/IA_Interact`
  (params (ActionValue :type Boolean) (ElapsedSeconds :type "Float (double-precision)") (TriggeredSeconds :type "Float (double-precision)") (InputAction :type "InputAction Object Reference" :default "/Game/Inputs/InputActions/IA_Interact.IA_Interact"))
  (:`Started`
    (bind _asl1_gamemode (cast `/Game/Blueprints/Level1/L1_Gamemode` (`GameplayStatics.GetGameMode`)))
    (set `/Game/Blueprints/Level1/L1_Gamemode.PlayerInteract` true _asl1_gamemode))
  (:`Completed`
    (set `/Game/Blueprints/Level1/L1_Gamemode.PlayerInteract` false _asl1_gamemode)))

(event `ToggleInventory`
  (bind _returnvalue (`GameplayStatics.GetPlayerController` 0))
  (if (`self.canOpenInventory`)
    (if (not (`self.isInventoryOpen`))
      (set `self.isInventoryOpen` true)
      (`CharacterMovementComponent.DisableMovement` (`Character.CharacterMovement` (`GameplayStatics.GetPlayerCharacter` 0)))
      (`Controller.SetIgnoreLookInput` _returnvalue true)
      (set `PlayerController.bShowMouseCursor` true _returnvalue)
      (`Widget.SetVisibility` (`self.InventoryMenu`) "SelfHitTestInvisible")
      (`WidgetBlueprintLibrary.SetInputMode_UIOnlyEx` (`GameplayStatics.GetPlayerController` 0) (`self.InventoryMenu`)))))

(event `self.ReceiveTick`
  (params (DeltaSeconds :type "Float (single-precision)"))
  (bind _camera (`self.Camera`))
  (bind _crosshairdot (`self.CrossHairDOt`))
  (bind _returnvalue (`SceneComponent.K2_GetComponentLocation` _camera))
  (bind _returnvalue_2 (`Widget.IsInViewport` (`self.CrossHairDOt`)))
  (`self.CrossHairDOt`
    (:`then`
      (bind (_outhit _returnvalue_3) (`KismetSystemLibrary.LineTraceSingle` _returnvalue (+ _returnvalue (* (`SceneComponent.GetForwardVector` _camera) 500.0)) "TraceTypeQuery1"))
      (if _returnvalue_3
        (bind (_bblockinghit _binitialoverlap _time _distance _location _impactpoint _normal _impactnormal _physmat _hitactor) (`GameplayStatics.BreakHitResult` _outhit))
        (if (or (`KismetSystemLibrary.DoesImplementInterface` _hitactor "/Script/HorrorGame.InterfaceInteract") (`KismetSystemLibrary.DoesImplementInterface` _hitactor "/Game/Blueprints/Interfaces/BPI_Interaction.BPI_Interaction_C"))
          (if (not _returnvalue_2)
            (`UserWidget.AddToViewport` _crosshairdot 0))
          (else
            (if _returnvalue_2 :!label _label
              (`Widget.RemoveFromParent` _crosshairdot))))
        (else
          (goto _label))))
    (:`else`)))

(event `Key|F`
  (params (Key :type "Key Structure"))
  (:`Pressed`
    (`FlashlightComponent.ToggleFlashlight` (`self.FlashlightComponent`))))

(event `CaughtByEnemies`
  (params (Enemy :type "Pawn Object Reference"))
  (`HealthComponent.RemoveHealth` (`self.Health`) 35.0)
  (`|ExecutionSequence`
    (:`then_0`
      (bind _asai_monster (cast `/Game/AI/MonsterAI/AI_Monster` Enemy))
      (`/Game/AI/MonsterAI/AI_Monster.KillPlayer` _asai_monster))
    (:`then_1`
      (bind _asai_zombie (cast `/Game/AI/ZombieAI/AI_Zombie` Enemy))
      (`/Game/AI/ZombieAI/AI_Zombie.KillPlayer` _asai_zombie))
    (:`then_2`
      (bind _asai_big_zombie (cast `/Game/AI/BigZombieAI/AI_BigZombie` Enemy))
      (`/Game/AI/BigZombieAI/AI_BigZombie.KillPlayer` _asai_big_zombie))))

(event `Key|Q`
  (params (Key :type "Key Structure"))
  (:`Pressed`
    (set `self.RotataLeft` false)
    (`self.InteractWithPuzzle` :!label _label_2)))

(event `Key|E`
  (params (Key :type "Key Structure"))
  (:`Pressed`
    (set `self.RotataLeft` true)
    (goto _label_2)))

(event `EnhancedInput|/Game/Inputs/InputActions/IA_Interact`
  (params (ActionValue :type Boolean) (ElapsedSeconds :type "Float (double-precision)") (TriggeredSeconds :type "Float (double-precision)") (InputAction :type "InputAction Object Reference" :default "/Game/Inputs/InputActions/IA_Interact.IA_Interact"))
  (bind _keypadinteract (`self.KeypadInteract`))
  (:`Started`
    (`/Engine/EditorBlueprintResources/StandardMacros.IsValid` _keypadinteract
      (:`Is Valid`
        (`/Game/Blueprints/Actors/Keypad/BP_Keypad.OnInteracted` _keypadinteract)))))

(fn `Initialize`
  (`|ExecutionSequence`
    (:`then_0`
      (bind _returnvalue (`|CreateWidget` "/Game/Widgets/WBP_Crosshair.WBP_Crosshair_C"))
      (set `self.CrossHairDOt` _returnvalue))
    (:`then_1`
      (bind _returnvalue_2 (`|CreateWidget` "/Game/Widgets/WBP_MainHUD.WBP_MainHUD_C"))
      (set `self.MAINHUD` _returnvalue_2))
    (:`then_2`
      (bind _returnvalue_3 (`|CreateWidget` "/Game/Widgets/Inventory/WBP_InventoryMenu.WBP_InventoryMenu_C"))
      (set `self.InventoryMenu` _returnvalue_3)
      (`Widget.SetVisibility` (`self.InventoryMenu`) "Collapsed"))
    (:`then_3`
      (`FlashlightComponent.Initialize` (`self.FlashlightComponent`) self))))

(fn `InteractWithPuzzle`
  (bind _camera (`self.Camera`))
  (bind _returnvalue (`SceneComponent.K2_GetComponentLocation` _camera))
  (bind (_outhit _returnvalue_2) (`KismetSystemLibrary.LineTraceSingle` _returnvalue (+ _returnvalue (* (`SceneComponent.GetForwardVector` _camera) 400)) "TraceTypeQuery1"))
  (if _returnvalue_2
    (bind (_bblockinghit _binitialoverlap _time _distance _location _impactpoint _normal _impactnormal _physmat _hitactor _hitcomponent) (`GameplayStatics.BreakHitResult` _outhit))
    (message `/Game/Blueprints/Interfaces/InteractPuzzle.InteractWithPuzzle` _hitactor _hitcomponent (`self.RotataLeft`))))

(fn `UserConstructionScript`)