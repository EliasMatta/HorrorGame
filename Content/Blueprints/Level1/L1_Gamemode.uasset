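; Level 1 game mode that manages persistent player settings and brings up the in-game UI.
; On BeginPlay it loads or creates the SaveSettings save object and copies mouse sensitivity and master volume onto HG_PlayerController.
; SaveGame writes those controller values back to the save slot.
; StartGame switches to game-only input, hides the cursor and adds L1_Character's main HUD and inventory menu to the viewport.
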(event `self.ReceiveBeginPlay`
  (bind _returnvalue (`GameplayStatics.DoesSaveGameExist` "SaveSettings"))
  (if _returnvalue
    (bind _returnvalue_2 (`GameplayStatics.LoadGameFromSlot` "SaveSettings"))
    (bind _assave_settings (cast `/Game/Settings/SaveSettings` _returnvalue_2))
    (bind _output_get (set `self.SaveSettingsREF` _assave_settings))
    (bind _ashg_player_controller (cast `/Game/Blueprints/HG_PlayerController` (`GameplayStatics.GetPlayerController` 0)))
    (set `PlayerControllerHG.LookSensitivity` (`/Game/Settings/SaveSettings.MouseSens` _output_get) _ashg_player_controller)
    (set `/Game/Blueprints/HG_PlayerController.MasterSlider` (`/Game/Settings/SaveSettings.SoundValue` _output_get) _ashg_player_controller)
    (else
      (bind _returnvalue_3 (`GameplayStatics.CreateSaveGameObject` "/Game/Settings/SaveSettings.SaveSettings_C"))
      (bind _output_get_2 (set `self.SaveSettingsREF` _returnvalue_3))
      (bind _ashg_player_controller_2 (cast `/Game/Blueprints/HG_PlayerController` (`GameplayStatics.GetPlayerController` 0)))
      (set `PlayerControllerHG.LookSensitivity` (`/Game/Settings/SaveSettings.MouseSens` _output_get_2) _ashg_player_controller_2)
      (set `/Game/Blueprints/HG_PlayerController.MasterSlider` (`/Game/Settings/SaveSettings.SoundValue` _output_get_2) _ashg_player_controller_2))))

(fn `Save Game`
  (bind _ashg_player_controller (cast `/Game/Blueprints/HG_PlayerController` (`GameplayStatics.GetPlayerController` 0)))
  (set `/Game/Settings/SaveSettings.MouseSens` (`PlayerControllerHG.LookSensitivity` _ashg_player_controller) (`self.SaveSettingsREF`))
  (set `/Game/Settings/SaveSettings.SoundValue` (`/Game/Blueprints/HG_PlayerController.MasterSlider` _ashg_player_controller) (`self.SaveSettingsREF`))
  (`GameplayStatics.SaveGameToSlot` (`self.SaveSettingsREF`) "SaveSettings"))

(fn `StartGame`
  (bind _returnvalue (`GameplayStatics.GetPlayerController` 0))
  (`WidgetBlueprintLibrary.SetInputMode_GameOnly` _returnvalue)
  (set `PlayerController.bShowMouseCursor` false _returnvalue)
  (bind _asl1_character (cast `/Game/Blueprints/Level1/L1_Character` (`GameplayStatics.GetPlayerCharacter` 0)))
  (`UserWidget.AddToViewport` (`/Game/Blueprints/Level1/L1_Character.MAINHUD` _asl1_character) 0)
  (bind _asl1_character_2 (cast `/Game/Blueprints/Level1/L1_Character` (`GameplayStatics.GetPlayerCharacter` 0)))
  (`UserWidget.AddToViewport` (`/Game/Blueprints/Level1/L1_Character.InventoryMenu` _asl1_character_2) 0))

(fn `UserConstructionScript`)